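; Game mode for field levels that spawns and possesses the player's field pawn when play begins.
; On BeginPlay it focuses the game viewport, then asks the game instance for the saved field position through an interface message.
; An empty saved level name places BP_FieldPlayer at the PlayerStart; otherwise it spawns at the last saved field transform, without comparing level names.
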(event `self.ReceiveBeginPlay`
  (`WidgetBlueprintLibrary.SetFocusToGameViewport`)
  (`self.SpawnPlayer`))

(fn `SpawnPlayer`
  (bind _playerfieldposition (message `/Game/Definitions/Interfaces/BPI_InstanceStorage.I_GetPlayerFieldPosition` (`GameplayStatics.GetGameInstance`)))
  (bind (_fieldlevelname _lastfieldtransform) (break `/Game/Definitions/Structs/S_FieldPosition` _playerfieldposition))
  (if (`KismetStringLibrary.IsEmpty` _fieldlevelname)
    (bind _returnvalue (`GameplayStatics.GetActorOfClass` "/Script/Engine.PlayerStart"))
    (bind (_returnvalue_location _returnvalue_rotation) (`KismetMathLibrary.BreakTransform` (`self.GetTransform` _returnvalue)))
    (bind _returnvalue_2 (`|SpawnActorFromClass` "/Game/Blueprints/Field/BP_FieldPlayer.BP_FieldPlayer_C" (`KismetMathLibrary.MakeTransform` _returnvalue_location _returnvalue_rotation) "Undefined" "MultiplyWithRoot" null null))
    (`Controller.Possess` (`GameplayStatics.GetPlayerController` 0) _returnvalue_2)
    (else
      (bind _returnvalue_3 (`|SpawnActorFromClass` "/Game/Blueprints/Field/BP_FieldPlayer.BP_FieldPlayer_C" (`KismetMathLibrary.MakeTransform` (.location _lastfieldtransform) (.rotation _lastfieldtransform)) "Undefined" "MultiplyWithRoot" null null))
      (`Controller.Possess` (`GameplayStatics.GetPlayerController` 0) _returnvalue_3))))

(fn `UserConstructionScript`)