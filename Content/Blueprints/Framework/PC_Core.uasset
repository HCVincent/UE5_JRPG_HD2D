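; PC_Core is a player controller Blueprint that creates and holds the HUD widgets for field and battle play.
; Interface events trigger InitWidgetField and InitWidgetBattle, which each create their widget owned by the controller, store it and add it to the viewport.
; Interface getters return the stored WBP_Field and WBP_Battle instances, so callers can reach them through the interface.
; BeginPlay and Tick are unused.
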(event `/Game/Definitions/Interfaces/BPI_UIControl.I_InitWidgetField`
  (`self.InitWidgetField`))

(event `/Game/Definitions/Interfaces/BPI_UIControl.I_InitWidgetBattle`
  (`self.InitWidgetBattle`))

(fn `I_GetWidgetBattle`
  (returns (WidgetBattle :type "/Game/UI/Widgets/WBP_Battle Object Reference"))
  (return (`self.WidgetBattle`)))

(fn `I_GetWidgetField`
  (returns (WidgetField :type "/Game/UI/Widgets/WBP_Field Object Reference"))
  (return (`self.WidgetField`)))

(fn `InitWidgetBattle`
  (bind _returnvalue (`|CreateWidget` "/Game/UI/Widgets/WBP_Battle.WBP_Battle_C" self))
  (bind _output_get (set `self.WidgetBattle` _returnvalue))
  (`UserWidget.AddToViewport` _output_get 0))

(fn `InitWidgetField`
  (bind _returnvalue (`|CreateWidget` "/Game/UI/Widgets/WBP_Field.WBP_Field_C" self))
  (bind _output_get (set `self.WidgetField` _returnvalue))
  (`UserWidget.AddToViewport` _output_get 0))

(fn `UserConstructionScript`)