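; Turn-based battle manager pawn that spawns warrior and slime teams, is possessed by the player and sways its camera yaw via a timeline.
; Turn order is party then enemies, with the front entry active and removed after its turn, and the list rebuilt when empty.
; Party members lerp to an active spot and back using timelines, while enemies just wait.
; No combat actions exist yet, only timed delays and debug prints.
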(event `self.ReceiveBeginPlay`
  (`self.StartBattle`))

(event `StartCameraSway`
  (bind _camera (`self.Camera`))
  (bind (_relativerotation_roll _relativerotation_pitch) (`KismetMathLibrary.BreakRotator` (`SceneComponent.RelativeRotation` _camera)))
  (`TimelineComponent.SetPlayRate` (`self.AnimCameraSway`) (`self.CameraSwayRate`))
  (bind (_direction _yawrotation) (`Timeline|AnimCameraSway` :!via `PlayFromStart`)
    (:`Update`
      (`SceneComponent.K2_SetRelativeRotation` _camera (`KismetMathLibrary.MakeRotator` _relativerotation_roll _relativerotation_pitch (* _yawrotation (`self.CameraSwayDistance`))) false false))))

(event `StartBattle`
  (for _array_element (`self.EnemyTeamLocations_0`)
    (bind _returnvalue (`|SpawnActorFromClass` "/Game/Blueprints/Battle/BattleChars/Enemies/Slime/BP_BattleSlime.BP_BattleSlime_C" (`KismetMathLibrary.MakeTransform` (+ _array_element (`self.SpawnHeightOffset`) (`self.K2_GetActorLocation`))) "AlwaysSpawn" "MultiplyWithRoot" null null))
    (`KismetArrayLibrary.Array_AddUnique` (`self.EnemyTeam`) _returnvalue))
  (for _array_element_2 (`self.PartyTeamLocations`)
    (bind _returnvalue_2 (`|SpawnActorFromClass` "/Game/Blueprints/Battle/BattleChars/Party/Warrior/BP_BattleWarrior.BP_BattleWarrior_C" (`KismetMathLibrary.MakeTransform` (+ _array_element_2 (`self.SpawnHeightOffset`) (`self.K2_GetActorLocation`)) (`self.PartyTeamRotation`)) "AlwaysSpawn" "MultiplyWithRoot" null null))
    (`KismetArrayLibrary.Array_AddUnique` (`self.PartyTeam`) _returnvalue_2))
  (`self.DecideTurnOrder`)
  (`self.SelectActiveCharacter`)
  (`self.StartCameraSway`)
  (`Controller.Possess` (`GameplayStatics.GetPlayerController` 0) self)
  (`self.StartTurn`))

(event `StartTurn`
  (`KismetSystemLibrary.PrintString` (`KismetStringLibrary.Concat_StrStr` (`KismetSystemLibrary.GetDisplayName` (`self.ActiveCharacter`)) " is active"))
  (if (`/Game/Blueprints/Battle/BattleChars/BP_BattleChar_BASE.IsPartyMember` (`self.ActiveCharacter`))
    (`self.MoveToActive`)
    (else
      (`KismetSystemLibrary.Delay` 2.0)
      (`self.ConcludeTurn`))))

(event `ConcludeTurn`
  (`KismetArrayLibrary.Array_Remove` (`self.TurnOrder`))
  (if (`KismetArrayLibrary.Array_IsEmpty` (`self.TurnOrder`))
    (`self.DecideTurnOrder`)
    (`self.SelectActiveCharacter`)
    (`self.StartTurn`)
    (else
      (`self.SelectActiveCharacter`)
      (`self.StartTurn`))))

(event `MoveToActive`
  ;[0.9427 0.6938 0 0.5] MoveToActive
  (`TimelineComponent.SetPlayRate` (`self.AnimMoveToActive`) 2.0) ; TODO get rid of magic number
  (bind (_direction _alpha) (`Timeline|AnimMoveToActive` :!via `PlayFromStart`)
    (:`Update`
      (`self.K2_SetActorLocation` (`self.ActiveCharacter`) (`KismetMathLibrary.VLerp` (`/Game/Blueprints/Battle/BattleChars/BP_BattleChar_BASE.SpawnedLocation` (`self.ActiveCharacter`)) (`self.AdjustedActiveLocation`) _alpha) false false))
    (:`Finished`
      (`KismetSystemLibrary.Delay` 2.0)
      (`self.MoveBackFromActive`))))

(event `MoveBackFromActive`
  ;[0.9427 0.6938 0 0.5] MoveBackFromActive
  (`TimelineComponent.SetPlayRate` (`self.AnimMoveBackActive`) 2.0) ; TODO get rid of magic number
  (bind (_direction _alpha) (`Timeline|AnimMoveBackActive` :!via `PlayFromStart`)
    (:`Update`
      (`self.K2_SetActorLocation` (`self.ActiveCharacter`) (`KismetMathLibrary.VLerp` (`self.AdjustedActiveLocation`) (`/Game/Blueprints/Battle/BattleChars/BP_BattleChar_BASE.SpawnedLocation` (`self.ActiveCharacter`)) _alpha) false false))
    (:`Finished`
      (`KismetSystemLibrary.Delay` 1.0)
      (`self.ConcludeTurn`))))

(fn `DecideTurnOrder`
  (`KismetArrayLibrary.Array_Clear` (`self.TurnOrder`))
  (`KismetArrayLibrary.Array_Append` (`self.TurnOrder`) (`self.PartyTeam`))
  (`KismetArrayLibrary.Array_Append` (`self.TurnOrder`) (`self.EnemyTeam`))
  (`KismetSystemLibrary.PrintString` (`KismetStringLibrary.Conv_IntToString` (`KismetArrayLibrary.Array_Length` (`self.TurnOrder`)))))

(fn `SelectActiveCharacter`
  (set `self.ActiveCharacter` (`|GetArrayItem` (`self.TurnOrder`))))

(fn `UserConstructionScript`)